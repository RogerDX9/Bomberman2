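; Input handler for a two-player local Bomberman game, driving the pawns of player controllers 0 and 1 from separate input mappings.
; Axis events move each pawn along world forward and right.
; Bomb presses spawn a Bomb below the pawn, decrement its CharacterComponent count and copy explosion distance to the BombComponent.
; With remote-controlled bombs, a press spawns only when the count is at maximum, otherwise it sets the detonate flag.
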(event Input|ActionEvents|InputActionSpawnBomb1
  (params (Key :type Key%20Structure))
  (bind _returnvalue (Game|GetPlayerController 0))
  (bind _returnvalue_2 (Pawn|GetControlledPawn _returnvalue))
  (bind _returnvalue_3 (Actor|GetComponentbyClass _returnvalue_2 "/Script/Bomberman2.CharacterComponent"))
  ;[1 1 1] SpawnBomb
  (:Pressed
    (if (Variables|/Script/Bomberman2.CharacterComponent|Getm_bRemoteControlledBombs _returnvalue_3)
      (if (== (Variables|/Script/Bomberman2.CharacterComponent|Getm_MaxNbOfBombs _returnvalue_3) (Variables|/Script/Bomberman2.CharacterComponent|Getm_NbOfBombs _returnvalue_3))
        (bind _returnvalue_4 (Game|SpawnActorfromClass "/Game/Bomberman2/Blueprints/Bomb.Bomb_C" (Math|Conversions|ToTransform(Vector) (+ (Transformation|GetActorLocation _returnvalue_2) "0, 0,-90.000000")) "Undefined" _returnvalue_2 0 :!label _label))
        (bind _result (Math|Integer|DecrementInt (Variables|/Script/Bomberman2.CharacterComponent|Getm_NbOfBombs _returnvalue_3))
          (:%20%20
            (Variables|/Script/Bomberman2.CharacterComponent|Setm_NbOfBombs _returnvalue_3 _result)
            (Variables|/Script/Bomberman2.BombComponent|Setm_ExplosionDistance (Actor|GetComponentbyClass _returnvalue_4 "/Script/Bomberman2.BombComponent") (Variables|/Script/Bomberman2.CharacterComponent|Getm_ExplosionDistance _returnvalue_3))))
        (else
          (Variables|/Script/Bomberman2.CharacterComponent|Setm_bDetonate _returnvalue_3 true)))
      (elif (Math|Conversions|ToBoolean(Integer) (Variables|/Script/Bomberman2.CharacterComponent|Getm_NbOfBombs _returnvalue_3))
        (goto _label)))))

(event Input|ActionEvents|InputActionSpawnBomb
  (params (Key :type Key%20Structure))
  (bind _returnvalue (Game|GetPlayerController 1))
  (bind _returnvalue_2 (Pawn|GetControlledPawn _returnvalue))
  (bind _returnvalue_3 (Actor|GetComponentbyClass _returnvalue_2 "/Script/Bomberman2.CharacterComponent"))
  ;[1 1 1] SpawnBomb
  (:Pressed
    (if (Variables|/Script/Bomberman2.CharacterComponent|Getm_bRemoteControlledBombs _returnvalue_3)
      (if (== (Variables|/Script/Bomberman2.CharacterComponent|Getm_MaxNbOfBombs _returnvalue_3) (Variables|/Script/Bomberman2.CharacterComponent|Getm_NbOfBombs _returnvalue_3))
        (bind _returnvalue_4 (Game|SpawnActorfromClass "/Game/Bomberman2/Blueprints/Bomb.Bomb_C" (Math|Conversions|ToTransform(Vector) (+ (Transformation|GetActorLocation _returnvalue_2) "0, 0,-90.000000")) "Undefined" _returnvalue_2 0 :!label _label))
        (bind _result (Math|Integer|DecrementInt (Variables|/Script/Bomberman2.CharacterComponent|Getm_NbOfBombs _returnvalue_3))
          (:%20%20
            (Variables|/Script/Bomberman2.CharacterComponent|Setm_NbOfBombs _returnvalue_3 _result)
            (Variables|/Script/Bomberman2.BombComponent|Setm_ExplosionDistance (Actor|GetComponentbyClass _returnvalue_4 "/Script/Bomberman2.BombComponent") (Variables|/Script/Bomberman2.CharacterComponent|Getm_ExplosionDistance _returnvalue_3))))
        (else
          (Variables|/Script/Bomberman2.CharacterComponent|Setm_bDetonate _returnvalue_3 true)))
      (elif (Math|Conversions|ToBoolean(Integer) (Variables|/Script/Bomberman2.CharacterComponent|Getm_NbOfBombs _returnvalue_3))
        (goto _label)))))

(event Input|AxisEvents|InputAxisMoveRight1
  (params (AxisValue :type Float%20%28single-precision%29))
  (Pawn|Input|AddMovementInput (Pawn|GetControlledPawn (Game|GetPlayerController 0)) (Math|Vector|GetRightVector "0, 0, 0") AxisValue false))

(event Input|AxisEvents|InputAxisMoveForward1
  (params (AxisValue :type Float%20%28single-precision%29))
  (Pawn|Input|AddMovementInput (Pawn|GetControlledPawn (Game|GetPlayerController 0)) (Math|Vector|GetForwardVector "0, 0, 0") AxisValue false))

(event Input|AxisEvents|InputAxisMoveForward
  (params (AxisValue :type Float%20%28single-precision%29))
  (Pawn|Input|AddMovementInput (Pawn|GetControlledPawn (Game|GetPlayerController 1)) (Math|Vector|GetForwardVector "0, 0, 0") AxisValue false))

(event Input|AxisEvents|InputAxisMoveRight
  (params (AxisValue :type Float%20%28single-precision%29))
  (Pawn|Input|AddMovementInput (Pawn|GetControlledPawn (Game|GetPlayerController 1)) (Math|Vector|GetRightVector "0, 0, 0") AxisValue false))

(fn ConstructionScript)