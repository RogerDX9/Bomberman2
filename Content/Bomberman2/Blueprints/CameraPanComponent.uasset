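; Camera pan component for Bomberman2 that keeps a shared camera centred above two players.
; Every tick it finds all BM2Character actors, storing the index-zero actor's location as Player 2 and any other's as Player 1.
; It moves the camera to their midpoint, raised with their separation down to a minimum height, so it pulls back as they spread out.
; Only location is set, with no smoothing or rotation.
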(event EventTick
  (params (DeltaSeconds :type Float%20%28single-precision%29))
  (bind _outactors (Actor|GetAllActorsOfClass "/Game/Bomberman2/Blueprints/BM2Character.BM2Character_C"))
  (for (_array_element _array_index) _outactors
    (if (Math|Conversions|ToBoolean(Integer) _array_index)
      (Variables|Default|SetPLayer1Location (Transformation|GetActorLocation _array_element))
      (else
        (Variables|Default|SetPlayer2Location (Transformation|GetActorLocation _array_element)))))
  (Transformation|SetActorLocation (Variables|Default|GetCamera) (Math|Vector|MakeVector (.X (Math|Vector|BreakVector (+ (Variables|Default|GetPLayer1Location) (* (Math|Vector|Normalize (- (Variables|Default|GetPlayer2Location) (Variables|Default|GetPLayer1Location))) (* (Math|Vector|VectorLength (- (Variables|Default|GetPlayer2Location) (Variables|Default|GetPLayer1Location))) 0.5))))) (.Y (Math|Vector|BreakVector (+ (Variables|Default|GetPLayer1Location) (* (Math|Vector|Normalize (- (Variables|Default|GetPlayer2Location) (Variables|Default|GetPLayer1Location))) (* (Math|Vector|VectorLength (- (Variables|Default|GetPlayer2Location) (Variables|Default|GetPLayer1Location))) 0.5))))) (+ (.Z (Math|Vector|BreakVector (+ (Variables|Default|GetPLayer1Location) (* (Math|Vector|Normalize (- (Variables|Default|GetPlayer2Location) (Variables|Default|GetPLayer1Location))) (* (Math|Vector|VectorLength (- (Variables|Default|GetPlayer2Location) (Variables|Default|GetPLayer1Location))) 0.5))))) (Math|Float|Max(Float) (+ (Math|Vector|VectorLength (- (Variables|Default|GetPlayer2Location) (Variables|Default|GetPLayer1Location))) 1e+02) 8e+02))) false false))