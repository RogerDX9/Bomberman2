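; Game mode for a two-player Bomberman match that runs the round timer and ends the round when time expires or a character is blasted.
; BeginPlay seeds the GameInstance timer, shows the timer widget, and ensures a local second player exists, tinted black and named Player 2.
; Tick polls all characters, adds points for survivors to GameInstance scores when someone is blasted, then shows the win screen and pauses.
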(event EventBeginPlay
  (bind _returnvalue (Game|GetPlayerController 1))
  (bind _returnvalue_2 (Pawn|GetControlledPawn _returnvalue))
  (bind _asbm2game_instance (Utilities|Casting|CastToBM2GameInstance (Game|GetGameInstance)))
  (Variables|/Game/Bomberman2/Blueprints/BM2GameInstance.BM2GameInstance_C|SetTimer _asbm2game_instance (Variables|Default|GetMapTime))
  (bind _returnvalue_3 (UserInterface|CreateWidget "/Game/Bomberman2/Blueprints/MapTimer.MapTimer_C" (Game|GetPlayerController 0)))
  (UserInterface|Viewport|AddtoViewport _returnvalue_3 0)
  (if (Utilities|IsValid _returnvalue)
    (Rendering|Material|SetVectorParameterValueonMaterials (Actor|GetComponentbyClass _returnvalue_2 "/Script/Engine.SkeletalMeshComponent") "BodyColor" "0, 0, 0")
    (Variables|/Script/Bomberman2.CharacterComponent|Setm_Name (Actor|GetComponentbyClass _returnvalue_2 "/Script/Bomberman2.CharacterComponent") "Player 2")
    (else
      (bind _returnvalue_4 (Class|GameplayStatics|CreatePlayer -1))
      (Rendering|Material|SetVectorParameterValueonMaterials (Actor|GetComponentbyClass (Pawn|GetControlledPawn _returnvalue_4) "/Script/Engine.SkeletalMeshComponent") "BodyColor" "0, 0, 0")
      (Variables|/Script/Bomberman2.CharacterComponent|Setm_Name (Actor|GetComponentbyClass (Pawn|GetControlledPawn _returnvalue_4) "/Script/Bomberman2.CharacterComponent") "Player 2"))))

(event EventTick
  (params (DeltaSeconds :type Float%20%28single-precision%29))
  (Variables|Default|SetPlayer1Score 0)
  (Variables|Default|SetPlayer2Score 0)
  (bind _outactors (Actor|GetAllActorsOfClass "/Game/Bomberman2/Blueprints/BM2Character.BM2Character_C"))
  (for _array_element _outactors
    (if (Variables|/Script/Bomberman2.DestructibleComponent|Getm_bBlasted (Actor|GetComponentbyClass _array_element "/Script/Bomberman2.DestructibleComponent"))
      (bind _result (Math|Integer|IncrementInt (Variables|Default|GetScored))
        (:%20%20
          (Variables|Default|SetScored _result)))
      (elif (Utilities|Enum|Equal(Enum) (Variables|/Script/Bomberman2.CharacterComponent|Getm_Name (Actor|GetComponentbyClass _array_element "/Script/Bomberman2.CharacterComponent")) "Player 1")
        (bind _result_2 (Math|Integer|IncrementInt (Variables|Default|GetPlayer1Score))
          (:%20%20
            (Variables|Default|SetPlayer1Score _result_2)))
        (elif (Utilities|Enum|Equal(Enum) (Variables|/Script/Bomberman2.CharacterComponent|Getm_Name (Actor|GetComponentbyClass _array_element "/Script/Bomberman2.CharacterComponent")) "Player 2")
          (bind _result_3 (Math|Integer|IncrementInt (Variables|Default|GetPlayer2Score))
            (:%20%20
              (Variables|Default|SetPlayer2Score _result_3)))))))
  (bind _asbm2game_instance (Utilities|Casting|CastToBM2GameInstance (Game|GetGameInstance)))
  (bind _output_get (Variables|/Game/Bomberman2/Blueprints/BM2GameInstance.BM2GameInstance_C|SetTimer _asbm2game_instance (- (Variables|/Game/Bomberman2/Blueprints/BM2GameInstance.BM2GameInstance_C|GetTimer _asbm2game_instance) DeltaSeconds)))
  (if (< _output_get 0.0)
    (bind _returnvalue (UserInterface|CreateWidget "/Game/Bomberman2/Blueprints/WinScreen.WinScreen_C" (Game|GetPlayerController 0) :!label _label))
    (UserInterface|Viewport|AddtoViewport _returnvalue 0)
    (Game|SetGamePaused true)
    (elif (Math|Conversions|ToBoolean(Integer) (Variables|Default|GetScored))
      (Variables|/Game/Bomberman2/Blueprints/BM2GameInstance.BM2GameInstance_C|SetPlayer1Score _asbm2game_instance (+ (Variables|/Game/Bomberman2/Blueprints/BM2GameInstance.BM2GameInstance_C|GetPlayer1Score _asbm2game_instance) (Variables|Default|GetPlayer1Score)))
      (Variables|/Game/Bomberman2/Blueprints/BM2GameInstance.BM2GameInstance_C|SetPlayer2Score _asbm2game_instance (+ (Variables|/Game/Bomberman2/Blueprints/BM2GameInstance.BM2GameInstance_C|GetPlayer2Score _asbm2game_instance) (Variables|Default|GetPlayer2Score)))
      (goto _label))))

(fn ConstructionScript)