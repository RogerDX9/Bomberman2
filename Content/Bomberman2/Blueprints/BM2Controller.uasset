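; Bomberman controller Blueprint that handles movement and bomb input for two local players.
; Separate input bindings move the pawns of player controllers 0 and 1 along fixed world axes and call a shared SpawnBomb function.
; SpawnBomb spawns a Bomb below the pawn, decrements its CharacterComponent bomb count and copies over blast distance.
; With controlled blast, it spawns only at a full bomb count and otherwise sets the detonate flag.
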(event Input|ActionEvents|InputActionSpawnBomb1
  (params (Key :type Key%20Structure))
  (:Pressed
    (CallFunction|SpawnBomb (Pawn|GetControlledPawn (Game|GetPlayerController 0)))))

(event Input|ActionEvents|InputActionSpawnBomb
  (params (Key :type Key%20Structure))
  (:Pressed
    (CallFunction|SpawnBomb (Pawn|GetControlledPawn (Game|GetPlayerController 1)))))

(event Input|AxisEvents|InputAxisMoveRight1
  (params (AxisValue :type Float%20%28single-precision%29))
  (Pawn|Input|AddMovementInput (Pawn|GetControlledPawn (Game|GetPlayerController 0)) (Math|Vector|GetRightVector "0, 0, 0") AxisValue false))

(event Input|AxisEvents|InputAxisMoveForward1
  (params (AxisValue :type Float%20%28single-precision%29))
  (Pawn|Input|AddMovementInput (Pawn|GetControlledPawn (Game|GetPlayerController 0)) (Math|Vector|GetForwardVector "0, 0, 0") AxisValue false))

(event Input|AxisEvents|InputAxisMoveForward
  (params (AxisValue :type Float%20%28single-precision%29))
  (Pawn|Input|AddMovementInput (Pawn|GetControlledPawn (Game|GetPlayerController 1)) (Math|Vector|GetForwardVector "0, 0, 0") AxisValue false))

(event Input|AxisEvents|InputAxisMoveRight
  (params (AxisValue :type Float%20%28single-precision%29))
  (Pawn|Input|AddMovementInput (Pawn|GetControlledPawn (Game|GetPlayerController 1)) (Math|Vector|GetRightVector "0, 0, 0") AxisValue false))

(fn ConstructionScript)

(fn SpawnBomb
  (params (Target :type Actor%20Object%20Reference))
  (bind _returnvalue (Actor|GetComponentbyClass Target "/Script/Bomberman2.CharacterComponent"))
  (if (Variables|/Script/Bomberman2.CharacterComponent|Getm_bControlledBlast _returnvalue)
    (if (== (Variables|/Script/Bomberman2.CharacterComponent|Getm_MaxNbOfBombs _returnvalue) (Variables|/Script/Bomberman2.CharacterComponent|Getm_NbOfBombs _returnvalue))
      (bind _returnvalue_2 (Game|SpawnActorfromClass "/Game/Bomberman2/Blueprints/Bomb.Bomb_C" (Math|Conversions|ToTransform(Vector) (+ (Transformation|GetActorLocation Target) "0, 0,-90.000000")) "Undefined" Target 0 :!label _label))
      (bind _result (Math|Integer|DecrementInt (Variables|/Script/Bomberman2.CharacterComponent|Getm_NbOfBombs _returnvalue))
        (:%20%20
          (Variables|/Script/Bomberman2.CharacterComponent|Setm_NbOfBombs _returnvalue _result)
          (Variables|/Script/Bomberman2.BombComponent|Setm_BlastDistance (Actor|GetComponentbyClass _returnvalue_2 "/Script/Bomberman2.BombComponent") (Variables|/Script/Bomberman2.CharacterComponent|Getm_BlastDistance _returnvalue))))
      (else
        (Variables|/Script/Bomberman2.CharacterComponent|Setm_bDetonateSpawnedBomb _returnvalue true)))
    (elif (Math|Conversions|ToBoolean(Integer) (Variables|/Script/Bomberman2.CharacterComponent|Getm_NbOfBombs _returnvalue))
      (goto _label))))