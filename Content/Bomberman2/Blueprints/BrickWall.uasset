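; BrickWall is a Bomberman-style wall that can drop a power-up when destroyed.
; On Destroyed, a weighted 30% roll decides whether a pickup spawns slightly below the wall's location.
; A chain of branches picks faster run, longer blast, more bombs or remote bomb.
; Each branch rolls a fresh random integer, so the odds are uneven and favour the fallback remote bomb.
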(event EventDestroyed
  (bind _returnvalue (Math|Random|RandomIntegerinRange 0 3))
  (bind _returnvalue_2 (Transformation|GetActorLocation))
  (bind _returnvalue_3 (+ _returnvalue_2 "0, 0,-30.000000"))
  (bind _returnvalue_4 (Math|Conversions|ToTransform(Vector) _returnvalue_3))
  (if (Math|Random|RandomBoolwithWeight 0.3)
    (if (== _returnvalue 0)
      (Game|SpawnActorfromClass "/Game/Bomberman2/Blueprints/FasterRunPickup.FasterRunPickup_C" _returnvalue_4 "Undefined" 0 0)
      (elif (== _returnvalue 1)
        (Game|SpawnActorfromClass "/Game/Bomberman2/Blueprints/LongerBlastPickup.LongerBlastPickup_C" _returnvalue_4 "Undefined" 0 0)
        (elif (== _returnvalue 2)
          (Game|SpawnActorfromClass "/Game/Bomberman2/Blueprints/MoreBombsPickup.MoreBombsPickup_C" _returnvalue_4 "Undefined" 0 0)
          (else
            (Game|SpawnActorfromClass "/Game/Bomberman2/Blueprints/RemoteBombPickup.RemoteBombPickup_C" _returnvalue_4 "Undefined" 0 0)))))))

(fn ConstructionScript)