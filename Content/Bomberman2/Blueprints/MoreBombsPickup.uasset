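; MoreBombsPickup is a Bomberman pickup that gives an extra bomb to whoever touches it.
; On BeginPlay it tints its static mesh green through the "Water Base Color" material parameter.
; When the mesh is overlapped by an actor with a CharacterComponent, it increments that component's current and maximum bomb counts, then destroys itself.
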(event OnComponentBeginOverlap(StaticMesh)
  (params (OverlappedComponent :type Primitive%20Component%20Object%20Reference) (OtherActor :type Actor%20Object%20Reference) (OtherComp :type Primitive%20Component%20Object%20Reference) (OtherBodyIndex :type Integer) (bFromSweep :type Boolean) (SweepResult :type Hit%20Result%20Structure%20%28by%20ref%29))
  (bind _returnvalue (Actor|GetComponentbyClass OtherActor "/Script/Bomberman2.CharacterComponent"))
  (if (Utilities|IsValid _returnvalue)
    (bind _result (Math|Integer|IncrementInt (Variables|/Script/Bomberman2.CharacterComponent|Getm_NbOfBombs _returnvalue))
      (:%20%20
        (Variables|/Script/Bomberman2.CharacterComponent|Setm_NbOfBombs _returnvalue _result)
        (bind _result_2 (Math|Integer|IncrementInt (Variables|/Script/Bomberman2.CharacterComponent|Getm_MaxNbOfBombs _returnvalue))
          (:%20%20
            (Variables|/Script/Bomberman2.CharacterComponent|Setm_MaxNbOfBombs _returnvalue _result_2)
            (Actor|DestroyActor)))))))

(event EventBeginPlay
  (Rendering|Material|SetVectorParameterValueonMaterials (Actor|GetComponentbyClass "/Script/Engine.StaticMeshComponent") "Water Base Color" "0,1.000000, 0"))

(fn ConstructionScript)